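; BP_SeedSpawner keeps a capped population of BP_Seed_Base actors spawned within its box bounds.
; On BeginPlay it attempts an initial batch and starts a looping cooldown timer for further spawns.
; Each attempt, while below the cap, picks a random point in the box and line traces vertically to place the seed on the hit surface.
; Spawned seeds are tracked in an array and removed through their OnDie event, freeing slots.
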(event `self.ReceiveBeginPlay`
  (`KismetSystemLibrary.K2_SetTimerDelegate` (delegate `SpawnSeed`) (`self.SpawnCooldown`) true)
  (for _ (range (`self.StartingAmountSpawned`))
    (`self.SpawnSeed`)))

(event `RemoveSeed`
  (params (`Dying Seed` :type "/Game/Gamejam/Functionality/Base/BP_Seed_Base Object Reference"))
  (`KismetArrayLibrary.Array_RemoveItem` (`self.SpawnedSeeds`) `Dying Seed`))

(event `SpawnSeed`
  (bind (_origin _boxextent) (`KismetSystemLibrary.GetComponentBounds` (`self.Box`)))
  (if (< (`KismetArrayLibrary.Array_Length` (`self.SpawnedSeeds`)) (`self.MaximumSeedsSpawned`))
    (bind _output_get (set `self.CurrentSpawningPoint` (`KismetMathLibrary.RandomPointInBoundingBox` _origin _boxextent)))
    (bind (_outhit _returnvalue) (`KismetSystemLibrary.LineTraceSingle` (+ _output_get (* (0.0 0.0 1.0) 500.0)) (+ _output_get (* (0.0 0.0 -1.0) 1000.0)) "TraceTypeQuery1"))
    (if _returnvalue
      (bind _returnvalue_2 (`|SpawnActorFromClass` "/Game/Gamejam/Functionality/Base/BP_Seed_Base.BP_Seed_Base_C" (`KismetMathLibrary.MakeTransform` (`.Location` (`GameplayStatics.BreakHitResult` _outhit))) "Undefined" "OverrideRootScale" null null))
      (`KismetArrayLibrary.Array_AddUnique` (`self.SpawnedSeeds`) _returnvalue_2)
      (add `/Game/Gamejam/Functionality/Base/BP_Seed_Base.OnDie` _returnvalue_2 (delegate `RemoveSeed`)))))

(fn `UserConstructionScript`)