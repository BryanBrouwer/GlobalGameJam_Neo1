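; BP_Turret_Dummy is a turret Blueprint whose only active logic spawns roots outward in eight directions.
; SpawnRoots loops over a 3x3 grid, skips the centre and passes each flat, unnormalized offset vector to SpawnRootTowards, which is defined outside this file.
; The event graph holds only disabled stubs and the construction script just calls the parent, so nothing here calls SpawnRoots.
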(fn `SpawnRoots`
  (for _index (range -1 2)
    (for _index_2 (range -1 2)
      (if (not (and (== _index_2 0) (== _index 0)))
        (`self.SpawnRootTowards` (`KismetMathLibrary.MakeVector` (`KismetMathLibrary.Conv_IntToDouble` _index_2) (`KismetMathLibrary.Conv_IntToDouble` _index)))))))

(fn `UserConstructionScript`
  (`parent.UserConstructionScript`))