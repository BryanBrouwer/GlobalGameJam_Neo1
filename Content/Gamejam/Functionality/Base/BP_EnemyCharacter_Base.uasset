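; Base enemy character that walks toward the home base, damages it on arrival and destroys itself.
; An enum state machine uses AI MoveTo, with box overlaps switching to root or home states; attacker enemies hit roots every second until RootIsDead.
; Damage is divided by armor and destroys the enemy at zero health.
; Debuffs include stackable Poison and Venom via recursive delayed events, plus slow, stuck and armor effects with explicit stop events.
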(event `self.ReceiveTick`
  (params (DeltaSeconds :type "Float (single-precision)"))
  ;[1 1 1] Debug code, you can remove
)

(event `self.ReceiveBeginPlay`
  (`self.MoveToHomeBase`))

(event `ApplyDebuff`
  (params (DebuffType :type "/Game/Gamejam/Functionality/Enums/E_EnemyDebuffs Enum" :default "NewEnumerator0") (Damage :type "Float (double-precision)") (Duration :type "Float (double-precision)") (DamageTimeInterval :type "Float (double-precision)"))
  (switch `/Game/Gamejam/Functionality/Enums/E_EnemyDebuffs` DebuffType
    (:`NewEnumerator0`
      (set `self.ApplyPoison` true)
      (set `self.PoisonRemainingTime` Duration)
      (`self.DebuffPoison` Damage DamageTimeInterval))
    (:`NewEnumerator5`
      (set `self.ApplyVenom` true)
      (set `self.VenomRemainingTime` Duration)
      (`self.DebuffVenom` Damage DamageTimeInterval))))

(event `RootIsDead`
  (set `self.IsAttackingRoot` false))

(event `SubtractHealth`
  (params (Damage :type "Float (double-precision)"))
  ;[1 1 1] Health and Death
  (bind _output_get (set `self.Health` (- (`self.Health`) (* Damage (/ 1.0 (`self.CurrentArmor`))))))
  (`KismetSystemLibrary.PrintString` (`KismetStringLibrary.Conv_DoubleToString` _output_get))
  (if (<= _output_get 0.0)
    (`self.K2_DestroyActor`)))

(event `DebuffPoison`
  (params (Damage :type "Float (double-precision)") (DamageTimeInterval :type "Float (double-precision)"))
  ;[1 0.3095 0.5029] Poison Debuff (applies damage once every certain amount of time passes)
  (if (`self.ApplyPoison`)
    (`self.SubtractHealth` Damage)
    (`KismetSystemLibrary.Delay` DamageTimeInterval)
    (bind _output_get (set `self.PoisonRemainingTime` (- (`self.PoisonRemainingTime`) DamageTimeInterval)))
    (if (> _output_get 0.0)
      (`self.DebuffPoison` Damage DamageTimeInterval)
      (else
        (set `self.ApplyPoison` false)))))

(event `self.BoxCollision.OnComponentBeginOverlap`
  (params (OverlappedComponent :type "PrimitiveComponent Object Reference") (OtherActor :type "Actor Object Reference") (OtherComp :type "PrimitiveComponent Object Reference") (OtherBodyIndex :type Integer) (bFromSweep :type Boolean) (SweepResult :type "HitResult Structure (by ref)"))
  ;[1 1 1] Overlap
  (`|ExecutionSequence`
    (:`then_0`
      (bind _asbp_root_base (cast `/Game/Gamejam/Functionality/Base/BP_Root_Base` OtherActor))
      (set `self.AttackTarget` _asbp_root_base)
      (set `self.EEnemyState` "NewEnumerator1")
      (`self.SwitchState`))
    (:`then_1`
      (cast `/Game/Gamejam/Functionality/BP_Home` OtherActor)
      (set `self.EEnemyState` "NewEnumerator3")
      (`self.SwitchState`))))

(event `DebuffVenom`
  (params (Damage :type "Float (double-precision)") (DamageInterval :type "Float (double-precision)"))
  ;[1 0.3095 0.5029] Venom Debuff. Same as poison, but can be applied at the same time as it, so it stacks
  (if (`self.ApplyVenom`)
    (`self.SubtractHealth` Damage)
    (`KismetSystemLibrary.Delay` DamageInterval)
    (bind _output_get (set `self.VenomRemainingTime` (- (`self.VenomRemainingTime`) DamageInterval)))
    (if (> _output_get 0.0)
      (`self.DebuffVenom` Damage DamageInterval)
      (else
        (set `self.ApplyVenom` false)))))

(event `BeginSlow`
  (params (SlowFactor :type "Float (double-precision)"))
  (bind _maxwalkspeed (`CharacterMovementComponent.MaxWalkSpeed` (`self.CharacterMovement`)))
  ;[1 0.3095 0.5029] Slow Debuff. Needs to call StopSlow for it to stop
  (set `self.SlowActive` true)
  (set `self.NormalMovementSpeed` _maxwalkspeed)
  (set `CharacterMovementComponent.MaxWalkSpeed` (* _maxwalkspeed SlowFactor) (`self.CharacterMovement`)))

(event `StopSlow`
  ;[1 0.3095 0.5029] Slow Debuff. Needs to call StopSlow for it to stop
  (if (`self.SlowActive`)
    (set `self.SlowActive` false)
    (set `CharacterMovementComponent.MaxWalkSpeed` 0.0 (`self.CharacterMovement`))))

(event `SwitchState`
  ;[0.2044 1 0.05729] State Machine
  (switch `/Game/Gamejam/Functionality/Enums/E_EnemyState` (`self.EEnemyState`)
    (:`NewEnumerator0`
      (`self.MoveToHomeBase`))
    (:`NewEnumerator1`
      (`self.MoveToRoots`))
    (:`NewEnumerator2`
      (`self.AttackRoots`))
    (:`NewEnumerator3`
      (`self.ReachedHomeBase`))))

(event `BeginArmorDebuff`
  (params (DebuffedArmor :type "Float (double-precision)"))
  ;[1 0.3095 0.5029] ArmorDebuff
  (set `self.ArmorDebuffActive` true)
  (set `self.CurrentArmor` DebuffedArmor))

(event `StopArmorDebuff`
  ;[1 0.3095 0.5029] ArmorDebuff
  (if (`self.ArmorDebuffActive`)
    (set `self.CurrentArmor` 1.0)))

(event `MoveToHomeBase`
  ;[0.5906 1 0.5149] Move to Home Bast
  (`|AIMoveTo` self (`SceneComponent.K2_GetComponentLocation` (`/Game/Gamejam/Functionality/BP_Home.DefaultSceneRoot` (`self.HomeTarget`))) null 0.1 true))

(event `BeginStuckDebuff`
  ;[1 0.3095 0.5029] Stuck Debuff. Needs to call StopStuckEvent for it to stop
  (set `self.StuckActive` true)
  (set `self.NormalMovementSpeed` (`CharacterMovementComponent.MaxWalkSpeed` (`self.CharacterMovement`)))
  (set `CharacterMovementComponent.MaxWalkSpeed` 0.0 (`self.CharacterMovement`)))

(event `StopStuckEvent`
  ;[1 0.3095 0.5029] Stuck Debuff. Needs to call StopStuckEvent for it to stop
  (if (`self.StuckActive`)
    (set `self.SlowActive` false)
    (set `CharacterMovementComponent.MaxWalkSpeed` (`self.NormalMovementSpeed`) (`self.CharacterMovement`))))

(event `MoveToRoots`
  ;[0.5906 1 0.5149] Move to Roots
  (if (`self.IsAttacker`)
    (`|AIMoveTo` self (`SceneComponent.K2_GetComponentLocation` (`/Game/Gamejam/Functionality/Base/BP_Root_Base.GFX_Placeholder` (`self.AttackTarget`))) null 1.0
      (:`OnSuccess`
        (set `self.EEnemyState` "NewEnumerator2"))
      (:`OnFail`
        (set `self.EEnemyState` "NewEnumerator0")))
    (`self.SwitchState`)))

(event `ReachedHomeBase`
  ;[0.5906 1 0.5149] Reached Home base and destroys itself
  (`/Game/Gamejam/Functionality/BP_Home.SubtractHealth` (`self.HomeTarget`) (`self.HomeDamage`))
  (`self.K2_DestroyActor`))

(event `AttackRoots`
  ;[0.5906 1 0.5149] Attack the Root
  (bind _output_get (set `self.IsAttackingRoot` true))
  (while _output_get
    (`/Game/Gamejam/Functionality/Base/BP_Root_Base.DamageRoot` (`self.AttackTarget`) (`self.AttackDamage`))
    (`KismetSystemLibrary.Delay` 1.0))
  (set `self.EEnemyState` "NewEnumerator0")
  (`self.SwitchState`))

(fn `UserConstructionScript`)