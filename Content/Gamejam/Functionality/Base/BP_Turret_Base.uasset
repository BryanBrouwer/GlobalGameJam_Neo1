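; Base turret actor that surrounds itself with roots on BeginPlay and can be damaged and destroyed.
; SpawnRoots walks a 3x3 grid minus the centre, spawning a RootClass actor at Range along each of the eight normalized directions, facing outward.
; Each root receives a reference to the turret and attaches to it, keeping its transform relative.
; TakeDamage sets Health to Amount minus Health (operands reversed from usual subtraction) and destroys the turret at zero or below.
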(event `self.ReceiveBeginPlay`
  (`self.SpawnRoots`))

(fn `ShouldSpawnRoot`
  (params (X :type Integer) (Y :type Integer))
  (returns (Spawn :type Boolean))
  (return (not (and (== X 0) (== Y 0)))))

(fn `SpawnRoots`
  (for _index (range -1 2)
    (for _index_2 (range -1 2)
      (bind _spawn (`self.ShouldSpawnRoot` _index_2 _index))
      (if _spawn
        (`self.SpawnRootTowards` (`KismetMathLibrary.MakeVector` (`KismetMathLibrary.Conv_IntToDouble` _index_2) (`KismetMathLibrary.Conv_IntToDouble` _index)))))))

(fn `SpawnRootTowards`
  (params (Direction :type "Vector Structure"))
  (bind _returnvalue (`|SpawnActorFromClass` (`self.RootClass`) (`KismetMathLibrary.MakeTransform` (* (`KismetMathLibrary.Normal` Direction) (`self.Range`)) (`KismetMathLibrary.Conv_VectorToRotator` Direction)) "Undefined" "OverrideRootScale" null 5.0 200.0 null))
  (`/Game/Gamejam/Functionality/Base/BP_Root_Base.SetTurret` _returnvalue self)
  (`self.K2_AttachToActor` _returnvalue self "None" "KeepRelative" "KeepRelative" "KeepRelative" true))

(fn `TakeDamage`
  (params (Amount :type "Float (double-precision)"))
  (bind _output_get (set `self.Health` (- Amount (`self.Health`))))
  (if (<= _output_get 0.0)
    (`self.K2_DestroyActor`)))

(fn `UserConstructionScript`)