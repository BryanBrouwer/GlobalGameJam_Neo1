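; Base seed actor that decays over time unless held, and can be planted to spawn a turret.
; On BeginPlay it picks a SeedType from a weighted table and starts the decay timer, which Interact pauses and SeedDropped resumes.
; Decay and PlantConfirm both fire OnDie and destroy the seed, with planting also spawning TurretType; PlantPreviewUpdate is empty.
; The construction script prints a warning unless table weights total 100.
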(event `self.ReceiveBeginPlay`
  (`self.GetRandomSeedType`)
  (`KismetSystemLibrary.PrintString` (`|GetEnumeratorNameAsString` (`self.SeedType`)))
  (bind _returnvalue (`KismetSystemLibrary.K2_SetTimerDelegate` (delegate `Decay`) (`self.DecayTime`)))
  (set `self.DecayTimer` _returnvalue))

(event `Decay`
  (`self.OnDie` self)
  (`self.K2_DestroyActor`))

(event `/Game/Gamejam/Functionality/Interface/BPI_InteractObject.Interact`
  (`KismetSystemLibrary.K2_PauseTimerHandle` (`self.DecayTimer`)))

(event `SeedDropped`
  (`KismetSystemLibrary.K2_UnPauseTimerHandle` (`self.DecayTimer`)))

(event `Plant Preview Update`
  (params (Location :type "Vector Structure")))

(event `Plant Confirm`
  (params (Location :type "Vector Structure") (Rotation :type "Rotator Structure"))
  (`self.OnDie` self)
  (`|SpawnActorFromClass` (`self.Turret Type`) (`KismetMathLibrary.MakeTransform` Location Rotation) "Undefined" "OverrideRootScale" null null)
  (`self.K2_DestroyActor`))

(fn `GetRandomSeedType`
  (locals (RandomValue :type Integer))
  (set `local.RandomValue` (`KismetMathLibrary.RandomIntegerInRange` 0 100))
  (for _array_element (`self.RandomSeedTable`)
    (bind _returnvalue (- (`local.RandomValue`) (`.Weight_6_9D4F43404839DD053516ED9372578FDC` (break `/Game/Gamejam/Functionality/Structs/F_SeedSpawningWeight` _array_element))))
    (set `local.RandomValue` _returnvalue)
    (if (<= _returnvalue 0)
      (set `self.SeedType` (break `/Game/Gamejam/Functionality/Structs/F_SeedSpawningWeight` _array_element))
      (break))))

(fn `UserConstructionScript`
  (locals (CurrentPercentageCombination :type Integer))
  (for _array_element (`self.RandomSeedTable`)
    (set `local.CurrentPercentageCombination` (+ (`.Weight_6_9D4F43404839DD053516ED9372578FDC` (break `/Game/Gamejam/Functionality/Structs/F_SeedSpawningWeight` _array_element)) (`local.CurrentPercentageCombination`))))
  (if (not (== (`local.CurrentPercentageCombination`) 100))
    (`KismetSystemLibrary.PrintString` (`KismetStringLibrary.Concat_StrStr` (`KismetSystemLibrary.GetObjectName` self) ": combined percentage is not 100!!!!!!") true true (struct :`R` 0.989583 :`B` 0.013596 :`A` 1.0) 20.0)))