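; Base actor for turret roots that attack enemies within a range sphere and forward damage to their parent turret.
; Overlap events track enemy capsules in ID-keyed maps, with hooks for entering and exiting.
; Once fully spawned, Tick runs per-enemy cooldowns and calls Attack, which here only prints.
; Logic to merge two overlapping roots into BP_RootCombined exists but is disconnected, and AddCombinationData is empty.
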(event `self.ReceiveBeginPlay`
  (`SphereComponent.SetSphereRadius` (`self.RangeCollider`) (`self.Range`) true)
  (`SphereComponent.SetSphereRadius` (`self.CombineColllider`) (`self.CombineRange`) true)
  (`KismetSystemLibrary.Delay` 0.1)
  (set `self.DetectCombineOverlap` false))

(event `self.ReceiveTick`
  (params (DeltaSeconds :type "Float (single-precision)"))
  (bind _enemynexthittime (`self.EnemyNextHitTime`))
  ;[1 1 1] Go through all enemies in range, check how much time has passed since last attack, and attack him if the cooldown has passed
  (if (`self.FullySpawned`)
    (bind _keys (`BlueprintMapLibrary.Map_Keys` (`self.EnemiesInRange`)))
    (for _array_element _keys
      (bind _value (`BlueprintMapLibrary.Map_Find` (`self.EnemyNextHitTime`) _array_element))
      (if (<= _value 0.0)
        (`self.Attack` (`BlueprintMapLibrary.Map_Find` (`self.EnemiesInRange`) _array_element))
        (`BlueprintMapLibrary.Map_Add` _enemynexthittime _array_element (`self.AttackCooldown`))
        (else
          (`BlueprintMapLibrary.Map_Add` _enemynexthittime _array_element (- _value DeltaSeconds)))))))

(event `self.RangeCollider.OnComponentBeginOverlap`
  (params (OverlappedComponent :type "PrimitiveComponent Object Reference") (OtherActor :type "Actor Object Reference") (OtherComp :type "PrimitiveComponent Object Reference") (OtherBodyIndex :type Integer) (bFromSweep :type Boolean) (SweepResult :type "HitResult Structure (by ref)"))
  ;[1 1 1] When an enemy enters range, add him to the map & set the lastHitTime for it to a negative value (so that he can be hit on the next Tick)
  (bind _asbp_enemy_character_base (cast `/Game/Gamejam/Functionality/Base/BP_EnemyCharacter_Base` OtherActor))
  (cast `CapsuleComponent` OtherComp)
  (bind _id (`/Game/Gamejam/Functionality/Base/BP_EnemyCharacter_Base.ID` _asbp_enemy_character_base))
  (`BlueprintMapLibrary.Map_Add` (`self.EnemiesInRange`) _id _asbp_enemy_character_base)
  (`BlueprintMapLibrary.Map_Add` (`self.EnemyNextHitTime`) _id)
  (`self.OnEnemyEnteredRange` _asbp_enemy_character_base))

(event `OnEnemyEnteredRange`
  (params (Enemy :type "/Game/Gamejam/Functionality/Base/BP_EnemyCharacter_Base Object Reference")))

(event `OnEnemyExitRange`
  (params (Enemy :type "/Game/Gamejam/Functionality/Base/BP_EnemyCharacter_Base Object Reference")))

(event `self.RangeCollider.OnComponentEndOverlap`
  (params (OverlappedComponent :type "PrimitiveComponent Object Reference") (OtherActor :type "Actor Object Reference") (OtherComp :type "PrimitiveComponent Object Reference") (OtherBodyIndex :type Integer))
  ;[1 1 1] When an enemy exits range, remove him from the two lists
  (bind _asbp_enemy_character_base (cast `/Game/Gamejam/Functionality/Base/BP_EnemyCharacter_Base` OtherActor))
  (cast `CapsuleComponent` OtherComp)
  (bind _id (`/Game/Gamejam/Functionality/Base/BP_EnemyCharacter_Base.ID` _asbp_enemy_character_base))
  (`BlueprintMapLibrary.Map_Remove` (`self.EnemiesInRange`) _id)
  (`BlueprintMapLibrary.Map_Remove` (`self.EnemyNextHitTime`) _id)
  (`self.OnEnemyExitRange` _asbp_enemy_character_base))

(event `DamageRoot`
  (params (Damage :type "Float (double-precision)"))
  (`/Game/Gamejam/Functionality/Base/BP_Turret_Base.TakeDamage` (`self.ParentTurret`) Damage))

(event `SetTurret`
  (params (ParentTurret :type "/Game/Gamejam/Functionality/Base/BP_Turret_Base Object Reference"))
  (set `self.ParentTurret` ParentTurret))

(event `self.CombineColllider.OnComponentBeginOverlap`
  (params (OverlappedComponent :type "PrimitiveComponent Object Reference") (OtherActor :type "Actor Object Reference") (OtherComp :type "PrimitiveComponent Object Reference") (OtherBodyIndex :type Integer) (bFromSweep :type Boolean) (SweepResult :type "HitResult Structure (by ref)"))
  ;[1 1 1] Spawn combined root if overlapping with same root
)

(fn `AddCombinationData`)

(fn `Attack`
  (params (Enemy :type "/Game/Gamejam/Functionality/Base/BP_EnemyCharacter_Base Object Reference"))
  (`KismetSystemLibrary.PrintString` (`KismetStringLibrary.Concat_StrStr` "Attack" (`KismetSystemLibrary.GetDisplayName` Enemy))))

(fn `UserConstructionScript`)