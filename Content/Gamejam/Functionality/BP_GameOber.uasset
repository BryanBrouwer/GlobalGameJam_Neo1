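; BP_GameOber is a level actor that ends the game and returns to the main menu once every way manager has finished.
; On BeginPlay it binds to the GameOber dispatcher of each entry in its WayManagers array.
; Each broadcast increments a counter, and when the count reaches the array length it opens L_Menu.
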(event `self.ReceiveBeginPlay`
  (for _array_element (`self.WayManagers`)
    (add `/Game/Gamejam/Functionality/BP_WayManager.GameOber` _array_element (delegate `AddToCounter`))))

(event `AddToCounter`
  (`/Engine/EditorBlueprintResources/StandardMacros.IncrementInt` (`self.Counter`)
    (:`  `
      (if (>= (`self.Counter`) (`KismetArrayLibrary.Array_Length` (`self.WayManagers`)))
        (`GameplayStatics.OpenLevel` "L_Menu")))))

(fn `UserConstructionScript`)