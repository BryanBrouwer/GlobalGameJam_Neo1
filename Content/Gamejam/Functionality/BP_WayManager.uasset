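; BP_WayManager is a wave spawner actor that runs a timed sequence of enemy waves from BeginPlay.
; Each wave spawns its whole EnemyList at once at the manager's transform, passing each enemy a HomeTarget and an incrementing ID.
; After the wave's TimeTillNextWave delay it advances to the next wave, or calls CallGameOber once the index reaches the WaveList length.
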(event `self.ReceiveBeginPlay`
  (`self.SpawnWave`))

(event `NextWave`
  (`/Engine/EditorBlueprintResources/StandardMacros.IncrementInt` (`self.CurrentWave`)
    (:`  `
      (`self.SpawnWave`))))

(event `SpawnWave`
  (bind (_output_wavenumber _output_timetillnextwave _output_enemylist) (break `/Game/Gamejam/Functionality/Structs/F_Wave` (`|GetArrayItem` (`self.WaveList`) (`self.CurrentWave`))))
  (for _array_element _output_enemylist
    (`|SpawnActorFromClass` _array_element (`self.GetTransform` self) "AdjustIfPossibleButAlwaysSpawn" "OverrideRootScale" null (`self.HomeTarget`) (`self.IdCounter`) 500.0 null)
    (`/Engine/EditorBlueprintResources/StandardMacros.IncrementInt` (`self.IdCounter`)))
  (`KismetSystemLibrary.Delay` _output_timetillnextwave)
  (if (>= (`self.CurrentWave`) (`KismetArrayLibrary.Array_Length` (`self.WaveList`)))
    (`self.GameOber`)
    (else
      (`self.NextWave`))))

(fn `UserConstructionScript`)