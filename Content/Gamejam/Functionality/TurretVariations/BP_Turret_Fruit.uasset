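; Fruit turret variant that grows in with a dissolve effect and restricts the base turret's root spawning to diagonals.
; On BeginPlay it creates dynamic rose tree and flower materials for the cube, then two chained timelines dissolve the tree, then the flowers.
; When both finish, it flags the actor found by GetActorOfClass on RootClass as FullySpawned.
; The ShouldSpawnRoot override adds an equal-absolute-X-and-Y condition to the parent's check.
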(event `self.ReceiveBeginPlay`
  (`parent.ReceiveBeginPlay`)
  (`|ExecutionSequence`
    (:`then_0`
      (`SceneComponent.SetVisibility` (`self.Cube`) false false)
      (bind _returnvalue (`PrimitiveComponent.CreateDynamicMaterialInstance` (`self.Cube`) 0 "/Game/Gamejam/Art/Models/Rose/MI_RoseFlowers.MI_RoseFlowers" "None"))
      (set `self.FlowerMat` _returnvalue)
      (bind _returnvalue_2 (`PrimitiveComponent.CreateDynamicMaterialInstance` (`self.Cube`) 1 "/Game/Gamejam/Art/Models/Rose/MI_Rose.MI_Rose" "None"))
      (set `self.TreeMat` _returnvalue_2))
    (:`then_1`
      (`SceneComponent.SetVisibility` (`self.Cube`) true false)
      (`self.SpawnTower`))))

(event `SpawnTower`
  (bind (_direction _spawntime) (`Timeline|Timeline_0`)
    (:`Update`
      (`MaterialInstanceDynamic.SetScalarParameterValue` (`self.TreeMat`) "Dissolve Amount" _spawntime))
    (:`Finished`
      (bind (_direction_2 _flowerspawntime) (`Timeline|Timeline_1`)
        (:`Update`
          (`MaterialInstanceDynamic.SetScalarParameterValue` (`self.FlowerMat`) "Dissolve Amount" _flowerspawntime))
        (:`Finished`
          (bind _returnvalue (`GameplayStatics.GetActorOfClass` (`self.RootClass`)))
          (set `/Game/Gamejam/Functionality/Base/BP_Root_Base.FullySpawned` true _returnvalue))))))

(fn `ShouldSpawnRoot`
  (params (X :type Integer) (Y :type Integer))
  (returns (Spawn :type Boolean))
  (bind _spawn (`parent.ShouldSpawnRoot` X Y))
  (return (and _spawn (== (`KismetMathLibrary.Abs_Int` X) (`KismetMathLibrary.Abs_Int` Y)))))

(fn `UserConstructionScript`
  (`parent.UserConstructionScript`))