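; Cotton plant turret variant that grows in with a staged dissolve effect on BeginPlay.
; Creates dynamic materials for the mesh's parts, then chains three timelines to animate Dissolve Amount on bark, then needles, then flowers and cotton.
; Overrides ShouldSpawnRoot to narrow the parent's result to a specific X/Y pattern.
; The final root actor lookup leaves its FullySpawned setter unconnected.
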(event `self.ReceiveBeginPlay`
  (`parent.ReceiveBeginPlay`)
  (`|ExecutionSequence`
    (:`then_0`
      (`SceneComponent.SetVisibility` (`self.Cube`) false false)
      (`|ExecutionSequence`
        (:`then_0`
          (bind _returnvalue (`PrimitiveComponent.CreateDynamicMaterialInstance` (`self.Cube`) 0 "/Game/Gamejam/Art/Models/Rose/MI_RoseFlowers.MI_RoseFlowers" "None"))
          (set `self.Flowers` _returnvalue))
        (:`then_1`
          (bind _returnvalue_2 (`PrimitiveComponent.CreateDynamicMaterialInstance` (`self.Cube`) 1 "/Game/Gamejam/Art/Models/Rose/MI_Rose.MI_Rose" "None"))
          (set `self.Bark` _returnvalue_2))
        (:`then_2`
          (bind _returnvalue_3 (`PrimitiveComponent.CreateDynamicMaterialInstance` (`self.Cube`) 2 "/Game/Gamejam/Art/Models/Rose/MI_Rose.MI_Rose" "None"))
          (set `self.Needles` _returnvalue_3))
        (:`then_3`
          (bind _returnvalue_4 (`PrimitiveComponent.CreateDynamicMaterialInstance` (`self.Cube`) 3 "/Game/Gamejam/Art/Models/Rose/MI_Rose.MI_Rose" "None"))
          (set `self.Needles2` _returnvalue_4))
        (:`then_4`
          (bind _returnvalue_5 (`PrimitiveComponent.CreateDynamicMaterialInstance` (`self.Cube`) 4 "/Game/Gamejam/Art/Models/Rose/MI_Rose.MI_Rose" "None"))
          (set `self.Cotton` _returnvalue_5))))
    (:`then_1`
      (`SceneComponent.SetVisibility` (`self.Cube`) true false)
      (`self.SpawnTower`))))

(event `SpawnTower`
  (bind (_direction _spawntime) (`Timeline|Timeline_0`)
    (:`Update`
      (`MaterialInstanceDynamic.SetScalarParameterValue` (`self.Bark`) "Dissolve Amount" _spawntime))
    (:`Finished`
      (bind (_direction_2 _needlespawntime) (`Timeline|Timeline_1`)
        (:`Update`
          (`MaterialInstanceDynamic.SetScalarParameterValue` (`self.Needles`) "Dissolve Amount" _needlespawntime)
          (`MaterialInstanceDynamic.SetScalarParameterValue` (`self.Needles2`) "Dissolve Amount" _needlespawntime))
        (:`Finished`
          (bind (_direction_3 _time) (`Timeline|Timeline_2`)
            (:`Update`
              (`MaterialInstanceDynamic.SetScalarParameterValue` (`self.Flowers`) "Dissolve Amount" _time)
              (`MaterialInstanceDynamic.SetScalarParameterValue` (`self.Cotton`) "Dissolve Amount" _time))
            (:`Finished`
              (bind _returnvalue (`GameplayStatics.GetActorOfClass` (`self.RootClass`))))))))))

(fn `ShouldSpawnRoot`
  (params (X :type Integer) (Y :type Integer))
  (returns (Spawn :type Boolean))
  (bind _spawn (`parent.ShouldSpawnRoot` X Y))
  (return (and _spawn (or (and (== X 0) (== Y 1)) (and (!= X 0) (== Y -1))))))

(fn `UserConstructionScript`
  (`parent.UserConstructionScript`))