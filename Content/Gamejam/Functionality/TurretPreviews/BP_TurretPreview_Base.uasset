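; Base turret placement preview actor that shows a turret mesh and its surrounding roots in a shared override material.
; On BeginPlay it spawns RootClass actors in the eight grid directions around itself, each facing outward at Range distance and attached with relative transforms.
; It applies MaterialToUse to every material slot on its cube and on each root's placeholder mesh.
; DeleteRoots destroys the tracked root actors.
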(event `self.ReceiveBeginPlay`
  (bind _cube (`self.Cube`))
  (`self.SpawnRoots`)
  (for _index (range (`KismetArrayLibrary.Array_Length` (`MeshComponent.GetMaterials` _cube)))
    (`PrimitiveComponent.SetMaterial` _cube _index (`self.MaterialToUse`))))

(event `DeleteRoots`
  (for _array_element (`self.Roots`)
    (`/Engine/EditorBlueprintResources/StandardMacros.IsValid` _array_element
      (:`Is Valid`
        (`self.K2_DestroyActor` _array_element)))))

(fn `ShouldSpawnRoot`
  (params (X :type Integer) (Y :type Integer))
  (returns (Spawn :type Boolean))
  (return (not (and (== X 0) (== Y 0)))))

(fn `SpawnRoots`
  (for _index (range -1 2)
    (for _index_2 (range -1 2)
      (bind _spawn (`self.ShouldSpawnRoot` _index_2 _index))
      (if _spawn
        (`self.SpawnRootTowards` (`KismetMathLibrary.MakeVector` (`KismetMathLibrary.Conv_IntToDouble` _index_2) (`KismetMathLibrary.Conv_IntToDouble` _index)))))))

(fn `SpawnRootTowards`
  (params (Direction :type "Vector Structure"))
  (bind _returnvalue (`|SpawnActorFromClass` (`self.RootClass`) (`KismetMathLibrary.MakeTransform` (* (`KismetMathLibrary.Normal` Direction) (`self.Range`)) (`KismetMathLibrary.Conv_VectorToRotator` Direction)) "Undefined" "OverrideRootScale" null 1000.0 null))
  (`KismetArrayLibrary.Array_AddUnique` (`self.Roots`) _returnvalue)
  (`self.K2_AttachToActor` _returnvalue self "None" "KeepRelative" "KeepRelative" "KeepRelative" true)
  (bind _gfx_placeholder (`/Game/Gamejam/Functionality/Base/BP_RootPreview_Base.GFX_Placeholder` _returnvalue))
  (for _index (range (`KismetArrayLibrary.Array_Length` (`MeshComponent.GetMaterials` _gfx_placeholder)))
    (`PrimitiveComponent.SetMaterial` _gfx_placeholder _index (`self.MaterialToUse`))))

(fn `UserConstructionScript`)