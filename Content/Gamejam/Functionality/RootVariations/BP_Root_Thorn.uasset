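; BP_Root_Thorn is the Thorn root variation, a child Blueprint that damages enemies.
; Its Attack function subtracts its Damage value from the target enemy's health.
; AddCombinationData appends its root type and damage to the created element's CombinedRootTypes for root combining, with debug prints around the step.
; BeginPlay only calls the parent, and a leftover SapTree debug spawn is unconnected.
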(event `self.ReceiveBeginPlay`
  (`parent.ReceiveBeginPlay`))

(fn `AddCombinationData`
  (`KismetSystemLibrary.PrintString` "Here2")
  (`KismetArrayLibrary.Array_Add` (`/Game/Gamejam/Functionality/RootVariations/BP_RootCombined.CombinedRootTypes` (`self.CreatedElement`)) (make `/Game/Gamejam/Functionality/Structs/F_RootTypeData` (`self.RootType`) (`self.Damage`)))
  (`KismetSystemLibrary.PrintString` "Here3"))

(fn `Attack`
  (params (Enemy :type "/Game/Gamejam/Functionality/Base/BP_EnemyCharacter_Base Object Reference"))
  (`/Game/Gamejam/Functionality/Base/BP_EnemyCharacter_Base.SubtractHealth` Enemy (`self.Damage`)))

(fn `UserConstructionScript`
  (`parent.UserConstructionScript`))