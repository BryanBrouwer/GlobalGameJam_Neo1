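; BP_Root_Pitcher is a root variant, likely a pitcher plant, that traps one enemy at a time and damages it.
; Attack claims the incoming enemy when none is held or the stored reference is invalid, starting its stuck debuff and subtracting Damage.
; While a valid enemy is held, only calls with a matching ID deal damage, so other enemies are ignored.
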(fn `Attack`
  (params (Enemy :type "/Game/Gamejam/Functionality/Base/BP_EnemyCharacter_Base Object Reference"))
  (if (`self.HasEnemy`)
    (`/Engine/EditorBlueprintResources/StandardMacros.IsValid` (`self.EnemyReference`)
      (:`Is Valid`
        (if (== (`/Game/Gamejam/Functionality/Base/BP_EnemyCharacter_Base.ID` Enemy) (`/Game/Gamejam/Functionality/Base/BP_EnemyCharacter_Base.ID` (`self.EnemyReference`)))
          (`/Game/Gamejam/Functionality/Base/BP_EnemyCharacter_Base.SubtractHealth` (`self.EnemyReference`) (`self.Damage`) :!label _label)))
      (:`Is Not Valid`
        (set `self.HasEnemy` true :!label _label_2)
        (bind _output_get (set `self.EnemyReference` Enemy))
        (`/Game/Gamejam/Functionality/Base/BP_EnemyCharacter_Base.BeginStuckDebuff` _output_get)
        (goto _label)))
    (else
      (goto _label_2))))

(fn `UserConstructionScript`
  (`parent.UserConstructionScript`))