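; Tower-defense root actor that merges several root types and applies all their effects to enemies.
; AddCombinedRoot extends the type list, which range, Tick and Attack logic each switch over per entry.
; Range events toggle Sap Tree slow and Cotton armor debuffs; Rafflesia debuffs on entry and in timed area pulses.
; Attack handles Thorn damage, chance-based Fruit poison and Pitcher's single-target stuck damage.
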(event `self.AddCombinedRoot`
  (params (CombinedRootTypes :type "Array of /Game/Gamejam/Functionality/Structs/F_RootTypeData Structure (by ref)"))
  (for _array_element (`self.CombinedRootTypes`)
    (set `self.FoundIdentical` false)
    (for _array_element_2 CombinedRootTypes
      (if (!= (`KismetMathLibrary.Conv_ByteToInt` (`.RootType_2_452B992F4CDB4EE428763A9424875748` (break `/Game/Gamejam/Functionality/Structs/F_RootTypeData` _array_element_2))) (`KismetMathLibrary.Conv_ByteToInt` (`.RootType_2_452B992F4CDB4EE428763A9424875748` (break `/Game/Gamejam/Functionality/Structs/F_RootTypeData` _array_element))))
        (set `self.FoundIdentical` true)))
    (if (not (`self.FoundIdentical`))
      (`KismetArrayLibrary.Array_Add` CombinedRootTypes _array_element))))

(event `self.OnEnemyEnteredRange`
  (params (Enemy :type "/Game/Gamejam/Functionality/Base/BP_EnemyCharacter_Base Object Reference"))
  (for _array_element (`self.CombinedRootTypes`)
    (bind (_roottype _damage _slowfactor _attackduration _poisonduration _poisondamageinterval _poisonchance _debuffedarmor) (break `/Game/Gamejam/Functionality/Structs/F_RootTypeData` _array_element))
    (switch `/Game/Gamejam/Functionality/Enums/E_RootType` _roottype
      (:`NewEnumerator2`
        (`/Game/Gamejam/Functionality/Base/BP_EnemyCharacter_Base.BeginSlow` Enemy _slowfactor))
      (:`NewEnumerator3`
        (`/Game/Gamejam/Functionality/Base/BP_EnemyCharacter_Base.BeginArmorDebuff` Enemy _debuffedarmor))
      (:`NewEnumerator5`
        (`/Game/Gamejam/Functionality/Base/BP_EnemyCharacter_Base.ApplyDebuff` Enemy "NewEnumerator4" 0.0 _attackduration 0.0)))))

(event `self.OnEnemyExitRange`
  (params (Enemy :type "/Game/Gamejam/Functionality/Base/BP_EnemyCharacter_Base Object Reference"))
  (for _array_element (`self.CombinedRootTypes`)
    (switch `/Game/Gamejam/Functionality/Enums/E_RootType` (`.RootType_2_452B992F4CDB4EE428763A9424875748` (break `/Game/Gamejam/Functionality/Structs/F_RootTypeData` _array_element))
      (:`NewEnumerator2`
        (`/Game/Gamejam/Functionality/Base/BP_EnemyCharacter_Base.StopSlow` Enemy))
      (:`NewEnumerator3`
        (`/Game/Gamejam/Functionality/Base/BP_EnemyCharacter_Base.StopArmorDebuff` Enemy)))))

(event `self.ReceiveTick`
  (params (DeltaSeconds :type "Float (single-precision)"))
  (for _array_element (`self.CombinedRootTypes`)
    (bind (_roottype _damage _slowfactor _attackduration) (break `/Game/Gamejam/Functionality/Structs/F_RootTypeData` _array_element))
    (switch `/Game/Gamejam/Functionality/Enums/E_RootType` _roottype
      (:`NewEnumerator5`
        (if (`self.AttackActive`)
          (bind _output_get (set `self.AttackEndTime` (- (`self.AttackEndTime`) DeltaSeconds)))
          (if (<= _output_get 0.0)
            (set `self.AttackActive` false))
          (else
            (bind _output_get_2 (set `self.NextAttackTime` (- (`self.NextAttackTime`) DeltaSeconds)))
            (if (and (<= _output_get_2 0.0) (> (`BlueprintMapLibrary.Map_Length` (`self.EnemiesInRange`)) 0))
              (set `self.AttackActive` true)
              (set `self.AttackEndTime` _attackduration)
              (set `self.NextAttackTime` (+ _attackduration (`self.AttackCooldown`)))
              (bind _values (`BlueprintMapLibrary.Map_Values` (`self.EnemiesInRange`)))
              (for _array_element_2 _values
                (`/Game/Gamejam/Functionality/Base/BP_EnemyCharacter_Base.ApplyDebuff` _array_element_2 "NewEnumerator4" 0.0 _attackduration 0.0)))))))))

(fn `Attack`
  (params (Enemy :type "/Game/Gamejam/Functionality/Base/BP_EnemyCharacter_Base Object Reference"))
  (for _array_element (`self.CombinedRootTypes`)
    (bind (_roottype _damage _slowfactor _attackduration _poisonduration _poisondamageinterval _poisonchance) (break `/Game/Gamejam/Functionality/Structs/F_RootTypeData` _array_element))
    (switch `/Game/Gamejam/Functionality/Enums/E_RootType` _roottype
      (:`NewEnumerator0`
        (`/Game/Gamejam/Functionality/Base/BP_EnemyCharacter_Base.SubtractHealth` Enemy _damage)
        (`KismetSystemLibrary.PrintString` "Thorn"))
      (:`NewEnumerator1`
        (if (<= (`KismetMathLibrary.RandomFloat`) _poisonchance)
          (`/Game/Gamejam/Functionality/Base/BP_EnemyCharacter_Base.ApplyDebuff` Enemy "NewEnumerator0" _damage _poisonduration _poisondamageinterval)))
      (:`NewEnumerator4`
        (if (`self.HasEnemy`)
          (`/Engine/EditorBlueprintResources/StandardMacros.IsValid` (`self.EnemyReference`)
            (:`Is Valid`
              (if (== (`/Game/Gamejam/Functionality/Base/BP_EnemyCharacter_Base.ID` Enemy) (`/Game/Gamejam/Functionality/Base/BP_EnemyCharacter_Base.ID` (`self.EnemyReference`)))
                (`/Game/Gamejam/Functionality/Base/BP_EnemyCharacter_Base.SubtractHealth` (`self.EnemyReference`) _damage :!label _label)))
            (:`Is Not Valid`
              (set `self.HasEnemy` true :!label _label_2)
              (bind _output_get (set `self.EnemyReference` (`self.EnemyReference`)))
              (`/Game/Gamejam/Functionality/Base/BP_EnemyCharacter_Base.BeginStuckDebuff` _output_get)
              (goto _label)))
          (else
            (goto _label_2)))))))

(fn `UserConstructionScript`
  (`parent.UserConstructionScript`))