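; BP_Root_Cotton is a root variation that debuffs enemy armor instead of attacking, with Attack deliberately left empty.
; Once fully spawned, it starts the armor debuff on enemies entering range and stops it when they exit.
; AddCombinedRoot appends its type and debuff value to a combined-root list only if no entry has a different type, despite the flag being named FoundIdentical.
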(event `self.OnEnemyEnteredRange`
  (params (Enemy :type "/Game/Gamejam/Functionality/Base/BP_EnemyCharacter_Base Object Reference"))
  (if (`self.FullySpawned`)
    (`/Game/Gamejam/Functionality/Base/BP_EnemyCharacter_Base.BeginArmorDebuff` Enemy (`self.DebuffedArmor`))))

(event `self.OnEnemyExitRange`
  (params (Enemy :type "/Game/Gamejam/Functionality/Base/BP_EnemyCharacter_Base Object Reference"))
  (if (`self.FullySpawned`)
    (`/Game/Gamejam/Functionality/Base/BP_EnemyCharacter_Base.StopArmorDebuff` Enemy)))

(event `self.AddCombinedRoot`
  (params (CombinedRootTypes :type "Array of /Game/Gamejam/Functionality/Structs/F_RootTypeData Structure (by ref)"))
  (bind _roottype (`self.RootType`))
  (set `self.FoundIdentical` false)
  (for _array_element CombinedRootTypes
    (if (!= (`KismetMathLibrary.Conv_ByteToInt` (`.RootType_2_452B992F4CDB4EE428763A9424875748` (break `/Game/Gamejam/Functionality/Structs/F_RootTypeData` _array_element))) (`KismetMathLibrary.Conv_ByteToInt` _roottype))
      (set `self.FoundIdentical` true)))
  (if (not (`self.FoundIdentical`))
    (`KismetArrayLibrary.Array_Add` CombinedRootTypes (make `/Game/Gamejam/Functionality/Structs/F_RootTypeData` _roottype 0.0 0.0 0.0 0.0 0.0 0.0 (`self.DebuffedArmor`)))))

(fn `Attack`
  (params (Enemy :type "/Game/Gamejam/Functionality/Base/BP_EnemyCharacter_Base Object Reference"))
  ;[1 1 1] Leave empty
)

(fn `UserConstructionScript`
  (`parent.UserConstructionScript`))