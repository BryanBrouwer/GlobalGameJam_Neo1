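; Rafflesia root variation that debuffs enemies within its range, with the single-target Attack left empty.
; Tick runs timed pulses that debuff all enemies in range, then counts down attack duration plus cooldown once each pulse ends.
; Entering enemies are debuffed immediately, whether or not a pulse is active.
; AddCombinedRoot appends this root's type and duration only if no listed entry has a differing type, despite the FoundIdentical name.
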(event `self.OnEnemyEnteredRange`
  (params (Enemy :type "/Game/Gamejam/Functionality/Base/BP_EnemyCharacter_Base Object Reference"))
  (`/Game/Gamejam/Functionality/Base/BP_EnemyCharacter_Base.ApplyDebuff` Enemy "NewEnumerator4" 0.0 (`self.AttackDuration`) 0.0))

(event `self.ReceiveTick`
  (params (DeltaSeconds :type "Float (single-precision)"))
  (bind _attackduration (`self.AttackDuration`))
  (if (`self.AttackActive`)
    (bind _output_get (set `self.AttackEndTime` (- (`self.AttackEndTime`) DeltaSeconds)))
    (if (<= _output_get 0.0)
      (set `self.AttackActive` false))
    (else
      (bind _output_get_2 (set `self.NextAttackTime` (- (`self.NextAttackTime`) DeltaSeconds)))
      (if (and (<= _output_get_2 0.0) (> (`BlueprintMapLibrary.Map_Length` (`self.EnemiesInRange`)) 0))
        (set `self.AttackActive` true)
        (set `self.AttackEndTime` _attackduration)
        (set `self.NextAttackTime` (+ _attackduration (`self.AttackCooldown`)))
        (bind _values (`BlueprintMapLibrary.Map_Values` (`self.EnemiesInRange`)))
        (for _array_element _values
          (`/Game/Gamejam/Functionality/Base/BP_EnemyCharacter_Base.ApplyDebuff` _array_element "NewEnumerator4" 0.0 (`self.AttackDuration`) 0.0))))))

(event `self.AddCombinedRoot`
  (params (CombinedRootTypes :type "Array of /Game/Gamejam/Functionality/Structs/F_RootTypeData Structure (by ref)"))
  (bind _roottype (`self.RootType`))
  (set `self.FoundIdentical` false)
  (for _array_element CombinedRootTypes
    (if (!= (`KismetMathLibrary.Conv_ByteToInt` (`.RootType_2_452B992F4CDB4EE428763A9424875748` (break `/Game/Gamejam/Functionality/Structs/F_RootTypeData` _array_element))) (`KismetMathLibrary.Conv_ByteToInt` _roottype))
      (set `self.FoundIdentical` true)))
  (if (not (`self.FoundIdentical`))
    (`KismetArrayLibrary.Array_Add` CombinedRootTypes (make `/Game/Gamejam/Functionality/Structs/F_RootTypeData` _roottype 0.0 0.0 (`self.AttackDuration`)))))

(fn `Attack`
  (params (Enemy :type "/Game/Gamejam/Functionality/Base/BP_EnemyCharacter_Base Object Reference"))
  ;[1 1 1] Leave empty
)

(fn `UserConstructionScript`
  (`parent.UserConstructionScript`))